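; BP_GameMode is a game mode that accepts player sessions when players log in to a dedicated server, apparently through GameLift.
; On InternalPreLogin it reads the playerid URL option and queries that player's sessions through the ServerObject held by BP_GameInstance.
; It accepts every returned session, with no branch that rejects the login when the lookup fails.
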(event `self.Internal_PreLogin`
  (params (Options :type String) (Address :type String) (ErrorMessage :type String))
  (if (`KismetSystemLibrary.IsDedicatedServer`)
    (bind _asbp_game_instance (cast `/Game/Blueprints/BP_GameInstance` (`GameplayStatics.GetGameInstance`)))
    (bind _serverobject (`/Game/Blueprints/BP_GameInstance.ServerObject` _asbp_game_instance)
      (:`then`
        (bind (_result _errortype _errormessage _returnvalue) (`GameLiftServerObject.DescribePlayerSessions` _serverobject (make `ServerDescribePlayerSessionsRequest` "" (`GameplayStatics.ParseOption` Options "playerid"))))
        (if _returnvalue
          (for _array_element (break `ServerDescribePlayerSessionsResult` _result)
            (`GameLiftServerObject.AcceptPlayerSession` _serverobject (`.PlayerSessionId` (break `ServerPlayerSession` _array_element))))))
      (:`else`))))

(fn `UserConstructionScript`)